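; Coffin box actor that sends the player back to where they began when they touch it.
; On BeginPlay it stores the player pawn's world location.
; When the collision component overlaps that pawn, it teleports the pawn to the stored location with a fixed facing.
; A disconnected sequence that would briefly hide a mesh and show a text render never runs.
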(event `self.ReceiveBeginPlay`
  (set `self.position` (`SceneComponent.K2_GetComponentLocation` (`Actor.RootComponent` (`GameplayStatics.GetPlayerPawn` 0)))))

(event `self.CollisionComp.OnComponentBeginOverlap`
  (params (OverlappedComponent :type "PrimitiveComponent Object Reference") (OtherActor :type "Actor Object Reference") (OtherComp :type "PrimitiveComponent Object Reference") (OtherBodyIndex :type Integer) (bFromSweep :type Boolean) (SweepResult :type "HitResult Structure (by ref)"))
  (bind _returnvalue (`GameplayStatics.GetPlayerPawn` 0))
  (if (== OtherActor _returnvalue)
    (`self.K2_SetActorLocationAndRotation` _returnvalue (`self.position`) (struct :`Yaw` -90.0) false true)))

(fn `UserConstructionScript`)