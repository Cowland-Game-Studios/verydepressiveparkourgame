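; Boulder trap actor that releases a physics boulder when its trigger is overlapped.
; The overlap shows the boulder and enables physics, then after two seconds hides it and disables physics and collision.
; The reset feeds the saved world location into a relative-location teleport.
; Any actor the boulder hits, with no filtering, is teleported to the world origin with zero rotation.
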(event `self.trigger.OnComponentBeginOverlap`
  (params (OverlappedComponent :type "PrimitiveComponent Object Reference") (OtherActor :type "Actor Object Reference") (OtherComp :type "PrimitiveComponent Object Reference") (OtherBodyIndex :type Integer) (bFromSweep :type Boolean) (SweepResult :type "HitResult Structure (by ref)"))
  (bind _bolder (`self.bolder`))
  (bind _bolder_2 (`self.bolder`))
  (set `self.location` (`SceneComponent.K2_GetComponentLocation` _bolder))
  (`SceneComponent.SetVisibility` _bolder true false)
  (`PrimitiveComponent.SetCollisionEnabled` (`self.bolder`) "PhysicsOnly")
  (`PrimitiveComponent.SetSimulatePhysics` (`self.bolder`) true)
  (`KismetSystemLibrary.Delay` 2.0)
  (`SceneComponent.K2_SetRelativeLocation` (`self.bolder`) (`self.location`) false true)
  (`SceneComponent.K2_SetRelativeLocation` _bolder_2 (`self.location`) false true)
  (`SceneComponent.SetVisibility` _bolder_2 false false)
  (`PrimitiveComponent.SetSimulatePhysics` _bolder_2 false)
  (`PrimitiveComponent.SetCollisionEnabled` (`self.bolder`) "NoCollision"))

(event `self.bolder.OnComponentHit`
  (params (HitComponent :type "PrimitiveComponent Object Reference") (OtherActor :type "Actor Object Reference") (OtherComp :type "PrimitiveComponent Object Reference") (NormalImpulse :type "Vector Structure") (Hit :type "HitResult Structure (by ref)"))
  (`self.K2_TeleportTo` :`self` OtherActor))

(fn `UserConstructionScript`)