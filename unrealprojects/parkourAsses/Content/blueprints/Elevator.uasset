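; Elevator actor with an automatic sliding door and a light that reacts to entering or leaving the room.
; Both begin and end overlap on EnterRoomDetectionBox toggle HouseLight visibility.
; OpenCloseDoor overlaps set the Open flag and start short Delay loops that teleport Door along X with growing per-step offsets.
; The shared MoveDoor counter sizes and bounds the steps, and flipping Open halts the opposing loop.
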(event `self.ReceiveBeginPlay`
  (set `self.MoveDoor` 0))

(event `self.EnterRoomDetectionBox.OnComponentBeginOverlap`
  (params (OverlappedComponent :type "PrimitiveComponent Object Reference") (OtherActor :type "Actor Object Reference") (OtherComp :type "PrimitiveComponent Object Reference") (OtherBodyIndex :type Integer) (bFromSweep :type Boolean) (SweepResult :type "HitResult Structure (by ref)"))
  (`SceneComponent.ToggleVisibility` (`self.HouseLight`) false :!label _label))

(event `self.EnterRoomDetectionBox.OnComponentEndOverlap`
  (params (OverlappedComponent :type "PrimitiveComponent Object Reference") (OtherActor :type "Actor Object Reference") (OtherComp :type "PrimitiveComponent Object Reference") (OtherBodyIndex :type Integer))
  (goto _label))

(event `self.OpenCloseDoor.OnComponentBeginOverlap`
  (params (OverlappedComponent :type "PrimitiveComponent Object Reference") (OtherActor :type "Actor Object Reference") (OtherComp :type "PrimitiveComponent Object Reference") (OtherBodyIndex :type Integer) (bFromSweep :type Boolean) (SweepResult :type "HitResult Structure (by ref)"))
  (bind _movedoor (`self.MoveDoor`))
  (set `self.Open` true)
  (`KismetSystemLibrary.Delay` 0.01 :!label _label_2)
  (if (and (< _movedoor 16) (== (`self.Open`) true))
    (`SceneComponent.K2_AddWorldOffset` (`self.Door`) (`KismetMathLibrary.Conv_IntVectorToVector` (make `IntVector` _movedoor)) false true)
    (bind _result (`/Engine/EditorBlueprintResources/StandardMacros.IncrementInt` _movedoor)
      (:`  `
        (set `self.MoveDoor` _result)
        (goto _label_2)))))

(event `self.OpenCloseDoor.OnComponentEndOverlap`
  (params (OverlappedComponent :type "PrimitiveComponent Object Reference") (OtherActor :type "Actor Object Reference") (OtherComp :type "PrimitiveComponent Object Reference") (OtherBodyIndex :type Integer))
  (bind _movedoor (`self.MoveDoor`))
  (set `self.Open` false)
  (`KismetSystemLibrary.Delay` 0.01 :!label _label_3)
  (if (and (> _movedoor 0) (== (`self.Open`) false))
    (`SceneComponent.K2_AddWorldOffset` (`self.Door`) (`KismetMathLibrary.Conv_IntVectorToVector` (make `IntVector` (- _movedoor 16))) false true)
    (bind _result (`/Engine/EditorBlueprintResources/StandardMacros.DecrementInt` _movedoor)
      (:`  `
        (set `self.MoveDoor` _result)
        (goto _label_3)))))

(fn `UserConstructionScript`)