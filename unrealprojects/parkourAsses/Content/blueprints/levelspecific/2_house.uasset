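; Level-specific house interaction actor that lets the player press F inside a trigger box to teleport to a hardcoded location.
; Box1 overlap enables actor input and shows a text prompt, while any actor overlap switches on a point light.
; F hides the shared root and its children, waits briefly, teleports the player pawn, then reuses the end-overlap logic to disable input and hide the text.
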(event `self.Box1.OnComponentBeginOverlap`
  (params (OverlappedComponent :type "PrimitiveComponent Object Reference") (OtherActor :type "Actor Object Reference") (OtherComp :type "PrimitiveComponent Object Reference") (OtherBodyIndex :type Integer) (bFromSweep :type Boolean) (SweepResult :type "HitResult Structure (by ref)"))
  (`self.EnableInput` (`GameplayStatics.GetPlayerController` 0))
  (`SceneComponent.SetVisibility` (`self.text`) true false))

(event `self.ReceiveActorBeginOverlap`
  (params (OtherActor :type "Actor Object Reference"))
  (`SceneComponent.SetVisibility` (`self.PointLight`) true false))

(event `self.Box1.OnComponentEndOverlap`
  (params (OverlappedComponent :type "PrimitiveComponent Object Reference") (OtherActor :type "Actor Object Reference") (OtherComp :type "PrimitiveComponent Object Reference") (OtherBodyIndex :type Integer))
  (`self.DisableInput` (`GameplayStatics.GetPlayerController` 0) :!label _label)
  (`SceneComponent.SetVisibility` (`self.text`) false false))

(event `Key|F`
  (params (Key :type "Key Structure"))
  (:`Pressed`
    (`SceneComponent.SetVisibility` (`self.SharedRoot`) false true)
    (`KismetSystemLibrary.Delay` 2.0)
    (`self.K2_TeleportTo` (`GameplayStatics.GetPlayerPawn` 0) (-2487.0 3544.0 3910.0) (struct))
    (goto _label)))

(fn `UserConstructionScript`)