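; Elevator portal that slides its door open as something approaches, then shuts it behind and loads another level.
; Two trigger overlaps drive zero-delay loops that offset the door along X each frame, stepping the shared Movedoor counter up or down to vary the speed.
; When closing brings the counter to 1, the current level's name selects an index into a hard-coded level list, and that level opens.
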(event `self.OpenDoor.OnComponentBeginOverlap`
  (params (OverlappedComponent :type "PrimitiveComponent Object Reference") (OtherActor :type "Actor Object Reference") (OtherComp :type "PrimitiveComponent Object Reference") (OtherBodyIndex :type Integer) (bFromSweep :type Boolean) (SweepResult :type "HitResult Structure (by ref)"))
  (bind _movedoor (`self.movedoor`))
  (`KismetSystemLibrary.Delay` 0.0 :!label _label)
  (if (< _movedoor 16)
    (`SceneComponent.K2_AddWorldOffset` (`self.door`) (`KismetMathLibrary.Conv_IntVectorToVector` (make `IntVector` _movedoor)) false true)
    (bind _result (`/Engine/EditorBlueprintResources/StandardMacros.IncrementInt` _movedoor)
      (:`  `
        (set `self.movedoor` _result)
        (goto _label)))))

(event `self.InsideCloseDoor.OnComponentBeginOverlap`
  (params (OverlappedComponent :type "PrimitiveComponent Object Reference") (OtherActor :type "Actor Object Reference") (OtherComp :type "PrimitiveComponent Object Reference") (OtherBodyIndex :type Integer) (bFromSweep :type Boolean) (SweepResult :type "HitResult Structure (by ref)"))
  (bind _movedoor (`self.movedoor`))
  (`KismetSystemLibrary.Delay` 0.0 :!label _label_2)
  (if (> _movedoor 0)
    (`SceneComponent.K2_AddWorldOffset` (`self.door`) (`KismetMathLibrary.Conv_IntVectorToVector` (make `IntVector` (- _movedoor 16))) false true)
    (bind _result (`/Engine/EditorBlueprintResources/StandardMacros.DecrementInt` _movedoor)
      (:`  `
        (set `self.movedoor` _result)
        (if (== _movedoor 1)
          (bind _returnvalue (`GameplayStatics.GetCurrentLevelName` true))
          (if (`KismetStringLibrary.EqualEqual_StrStr` _returnvalue "level1")
            (set `self.levelcount` 2)
            (elif (`KismetStringLibrary.EqualEqual_StrStr` _returnvalue "level2")
              (set `self.levelcount` 3)
              (elif (`KismetStringLibrary.EqualEqual_StrStr` _returnvalue "level3")
                (set `self.levelcount` 4)
                (elif (`KismetStringLibrary.EqualEqual_StrStr` _returnvalue "level43d")
                  (set `self.levelcount` 5)
                  (elif (`KismetStringLibrary.EqualEqual_StrStr` _returnvalue "level5")
                    (set `self.levelcount` 6)
                    (else
                      (set `self.levelcount` 1)))))))
          (`GameplayStatics.OpenLevel` (`|GetArrayItem` (`|MakeArray` "tutorial" "level5" "level2" "level3" "level4" "level1" "ending" "None" :!type "Name") (`self.levelcount`)) false)
          (else
            (goto _label_2)))))))

(fn `UserConstructionScript`)