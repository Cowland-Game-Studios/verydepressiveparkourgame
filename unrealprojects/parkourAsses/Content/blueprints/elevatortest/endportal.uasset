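; End portal Blueprint in an elevator test folder, with a door that closes and opens when trigger components are overlapped.
; InsideCloseDoor and OpenDoor overlaps run opposing zero-delay loops that shift the Door along world X once per frame, teleporting without sweep.
; Both loops share the Movedoor counter, which bounds the travel and sets each step's size, so the door accelerates in either direction.
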(event `self.InsideCloseDoor.OnComponentBeginOverlap`
  (params (OverlappedComponent :type "PrimitiveComponent Object Reference") (OtherActor :type "Actor Object Reference") (OtherComp :type "PrimitiveComponent Object Reference") (OtherBodyIndex :type Integer) (bFromSweep :type Boolean) (SweepResult :type "HitResult Structure (by ref)"))
  (bind _movedoor (`self.movedoor`))
  (`KismetSystemLibrary.Delay` 0.0 :!label _label)
  (if (< _movedoor 16)
    (`SceneComponent.K2_AddWorldOffset` (`self.door`) (`KismetMathLibrary.Conv_IntVectorToVector` (make `IntVector` _movedoor)) false true)
    (bind _result (`/Engine/EditorBlueprintResources/StandardMacros.IncrementInt` _movedoor)
      (:`  `
        (set `self.movedoor` _result)
        (goto _label)))))

(event `self.OpenDoor.OnComponentBeginOverlap`
  (params (OverlappedComponent :type "PrimitiveComponent Object Reference") (OtherActor :type "Actor Object Reference") (OtherComp :type "PrimitiveComponent Object Reference") (OtherBodyIndex :type Integer) (bFromSweep :type Boolean) (SweepResult :type "HitResult Structure (by ref)"))
  (bind _movedoor (`self.movedoor`))
  (`KismetSystemLibrary.Delay` 0.0 :!label _label_2)
  (if (> _movedoor 0)
    (`SceneComponent.K2_AddWorldOffset` (`self.door`) (`KismetMathLibrary.Conv_IntVectorToVector` (make `IntVector` (- _movedoor 16))) false true)
    (bind _result (`/Engine/EditorBlueprintResources/StandardMacros.DecrementInt` _movedoor)
      (:`  `
        (set `self.movedoor` _result)
        (goto _label_2)))))

(fn `UserConstructionScript`)